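; Keyboard tuning Blueprint for an nDisplay warp-mesh setup, adjusting the in-camera FOV multiplier at runtime.
; BeginPlay enables input, finds BP_WarpMonitor and caches the local viewport IDs from the DisplayCluster API.
; Add/Subtract step the FOV multiplier, Period nudges the monitor's root yaw, and 9 increments ExposureAMT and pushes camera post-process settings to each viewport.
; Tracker-driven offset and other rotation corrections are disconnected.
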(event EventBeginPlay
  ;[1 1 1] Setup
  (Input|EnableInput (Game|GetPlayerController 0))
  (Development|PrintString "FOV Input")
  (bind _returnvalue (Actor|GetActorOfClass "/Game/WarpMesh/BP_WarpMonitor.BP_WarpMonitor_C"))
  (Utilities|IsValid _returnvalue
    (:Is%20Valid
      (Variables|Default|SetMesh%20Wall _returnvalue)
      (bind _asdisplay_cluster_blueprint_apiimpl (Utilities|Casting|CastToDisplayClusterBlueprintAPIImpl (Class|DisplayClusterBlueprintLib|GetAPI)))
      (bind _viewportids (Class|DisplayClusterBlueprintAPIImpl|GetLocalViewports _asdisplay_cluster_blueprint_apiimpl false))
      (Variables|Default|SetViews _viewportids))))

(event Input|KeyboardEvents|T
  (params (Key :type Key%20Structure :default "None"))
  ;[1 1 1] T- Pos reset (possibly redundant?)
)

(event Input|KeyboardEvents|Add
  (params (Key :type Key%20Structure :default "None"))
  (bind _incamera (Variables|Default|GetIncamera))
  (:Pressed
    (Variables|/nDisplay/Blueprints/ReprojectionCamera/BP_IncameraSettings.BP_IncameraSettings_C|SetFOVMultiplier _incamera (+ (Variables|/nDisplay/Blueprints/ReprojectionCamera/BP_IncameraSettings.BP_IncameraSettings_C|GetFOVMultiplier _incamera) 0.1))))

(event Input|KeyboardEvents|Subtract
  (params (Key :type Key%20Structure :default "None"))
  (bind _incamera (Variables|Default|GetIncamera))
  (:Pressed
    (Variables|/nDisplay/Blueprints/ReprojectionCamera/BP_IncameraSettings.BP_IncameraSettings_C|SetFOVMultiplier _incamera (+ (Variables|/nDisplay/Blueprints/ReprojectionCamera/BP_IncameraSettings.BP_IncameraSettings_C|GetFOVMultiplier _incamera) -0.1))))

(event Input|KeyboardEvents|9
  (params (Key :type Key%20Structure :default "None"))
  (:Pressed
    (Variables|Default|SetexposureAMT (+ (Variables|Default|GetexposureAMT) 1.0))
    (bind _structout (Utilities|Struct|SetmembersinPostProcessSettings (Variables|/Script/Engine.CameraComponent|GetPostProcessSettings (Variables|/Script/Engine.CameraActor|GetCameraComponent (Variables|/nDisplay/Blueprints/ReprojectionCamera/BP_IncameraSettings.BP_IncameraSettings_C|GetReprojectedCineCamera (Variables|Default|GetIncamera))))))
    (bind _asdisplay_cluster_blueprint_apiimpl (Utilities|Casting|CastToDisplayClusterBlueprintAPIImpl (Class|DisplayClusterBlueprintLib|GetAPI)))
    (bind _array_element (Utilities|Array|ForEachLoopwithBreak (Variables|Default|GetViews))
      (:LoopBody
        (Class|DisplayClusterBlueprintAPIImpl|SetFinalPostProcessingSettings _asdisplay_cluster_blueprint_apiimpl _array_element _structout)
        (Development|PrintString "Updated post process settings")))))

(event Input|KeyboardEvents|Period
  (params (Key :type Key%20Structure :default "None"))
  (bind _mesh_wall (Variables|Default|GetMesh%20Wall))
  (bind _root_offset (Variables|/Game/WarpMesh/BP_WarpMonitor.BP_WarpMonitor_C|Getroot%20Offset _mesh_wall))
  ;[1 1 1] Root correction for projection Z rotation
  (:Pressed
    (Transformation|SetRelativeRotation _root_offset (Math|Rotator|MakeRotator 0.0 0.0 (+ (.yaw (Variables|/Script/Engine.SceneComponent|GetRelativeRotation _root_offset)) -0.5)) false false)))

(fn ConstructionScript)